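; BP_Mesh_Eraser is an actor whose Cube defines the erase region published to the MP_Erase Material Parameter Collection.
; It writes the Cube's world location and scale to the Location and Scale vector parameters in the Construction Script and again on BeginPlay.
; Rotation is not passed, runtime movement is not tracked, and multiple instances overwrite the same shared values.
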(event `self.ReceiveBeginPlay`
  (bind _cube (`self.Cube`))
  (`KismetMaterialLibrary.SetVectorParameterValue` "/Game/Blueprints/Cross_Section_View/MP_Erase.MP_Erase" "Location" (`KismetMathLibrary.Conv_VectorToLinearColor` (`SceneComponent.K2_GetComponentLocation` _cube)))
  (`KismetMaterialLibrary.SetVectorParameterValue` "/Game/Blueprints/Cross_Section_View/MP_Erase.MP_Erase" "Scale" (`KismetMathLibrary.Conv_VectorToLinearColor` (`SceneComponent.K2_GetComponentScale` _cube))))

(fn `UserConstructionScript`
  (bind _cube (`self.Cube`))
  (`KismetMaterialLibrary.SetVectorParameterValue` "/Game/Blueprints/Cross_Section_View/MP_Erase.MP_Erase" "Location" (`KismetMathLibrary.Conv_VectorToLinearColor` (`SceneComponent.K2_GetComponentLocation` _cube)))
  (`KismetMaterialLibrary.SetVectorParameterValue` "/Game/Blueprints/Cross_Section_View/MP_Erase.MP_Erase" "Scale" (`KismetMathLibrary.Conv_VectorToLinearColor` (`SceneComponent.K2_GetComponentScale` _cube))))