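; BP_Launch_Plane is a launched plane projectile that spawns a BP_Mesh_Eraser on impact.
; On BeginPlay it applies a large forward impulse to its Plane component.
; On hit, AddScale uses counting loops to derive whole-step extents from the hit actor's scale, stretched in X and Z and halved in Y.
; It spawns the eraser at the Plane's relative-transform location with that scale, then destroys itself.
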(event `self.ReceiveBeginPlay`
  (bind _plane (`self.Plane`))
  (`PrimitiveComponent.AddImpulse` _plane (* (`SceneComponent.GetForwardVector` _plane) 3000000) "None" false))

(event `self.ReceiveHit`
  (params (MyComp :type "PrimitiveComponent Object Reference") (Other :type "Actor Object Reference") (OtherComp :type "PrimitiveComponent Object Reference") (bSelfMoved :type Boolean) (HitLocation :type "Vector Structure") (HitNormal :type "Vector Structure") (NormalImpulse :type "Vector Structure") (Hit :type "HitResult Structure (by ref)"))
  (bind _returnvalue_location (`KismetMathLibrary.BreakTransform` (`SceneComponent.GetRelativeTransform` (`self.Plane`))))
  (`self.Add Scale`)
  (`|SpawnActorFromClass` "/Game/Blueprints/Cross_Section_View/BP_Mesh_Eraser.BP_Mesh_Eraser_C" (`KismetMathLibrary.MakeTransform` _returnvalue_location (struct) (`KismetMathLibrary.MakeVector` (`self.XDifference`) (`self.YDifference`) (`self.ZDifference`))) "Undefined" "MultiplyWithRoot" null null)
  (`self.K2_DestroyActor`))

(event `Add Scale`
  (bind _ydifference (`self.YDifference`))
  (bind _xdifference (`self.XDifference`))
  (bind _zdifference (`self.ZDifference`))
  (bind (_returnvalue_location _returnvalue_rotation _returnvalue_scale) (`KismetMathLibrary.BreakTransform` (`self.GetTransform` (stale `self.ReceiveHit` Other))))
  (bind (_returnvalue_x _returnvalue_y _returnvalue_z) (`KismetMathLibrary.BreakVector` (* _returnvalue_scale (2.0 0.5 2.0))))
  (while (< _ydifference _returnvalue_y)
    (set `self.YDifference` (+ _ydifference 1.0)))
  (`/Engine/EditorBlueprintResources/StandardMacros.IncrementFloat` _ydifference
    (:`  `
      (while (< _xdifference _returnvalue_x)
        (set `self.XDifference` (+ _xdifference 1.0)))
      (`/Engine/EditorBlueprintResources/StandardMacros.IncrementFloat` _xdifference
        (:`  `
          (while (< _zdifference _returnvalue_z)
            (set `self.ZDifference` (+ _zdifference 1.0)))
          (`/Engine/EditorBlueprintResources/StandardMacros.IncrementFloat` _zdifference))))))

(fn `UserConstructionScript`)